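; BP_musicBox is a music box actor, apparently for relaxation room audio, but none of its events are wired to logic.
; TriggerMusic and the Widget component's click and activation events are empty.
; Disconnected nodes would stop the level's AmbientSound, pick a random row from RelaxationRoomAudio_DataTable, play its audio in 2D and print its name, but never run.
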(event OnComponentActivated(Widget)
  (params (Component :type Actor%20Component%20Object%20Reference) (bReset :type Boolean)))

(event OnClicked(Widget)
  (params (TouchedComponent :type Primitive%20Component%20Object%20Reference) (ButtonPressed :type Key%20Structure :default "None")))

(event Custom|TriggerMusic)

(event EventBeginPlay)

(event Collision|EventActorBeginOverlap
  (params (OtherActor :type Actor%20Object%20Reference)))

(event EventTick
  (params (DeltaSeconds :type Float%20%28single-precision%29)))

(fn ConstructionScript)