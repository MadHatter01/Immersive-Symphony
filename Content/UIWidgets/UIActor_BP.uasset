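; Instrument exhibit actor that plays an instrument's music when something overlaps its Collision component.
; The placed actor's display name selects the Ukulele, Piano or Trumpet row from the instrument data table.
; MusicPlaying blocks repeat 2D playback until overlap ends, which resets the flag without stopping the sound.
; ExpandUIWidget receives the row but does nothing, as its text and button-filling nodes are disconnected.
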(event OnComponentBeginOverlap(collision)
  (params (OverlappedComponent :type Primitive%20Component%20Object%20Reference) (OtherActor :type Actor%20Object%20Reference) (OtherComp :type Primitive%20Component%20Object%20Reference) (OtherBodyIndex :type Integer) (bFromSweep :type Boolean) (SweepResult :type Hit%20Result%20Structure%20%28by%20ref%29))
  (switch string (Utilities|GetDisplayName (Components|GetOwner OverlappedComponent))
    (:UIActor_BP
      (Variables|Default|Setactorvalue "I0")
      (bind _returnvalue (Utilities|GetDataTableRow "/Game/Instrument_dataTable.Instrument_dataTable" "Ukulele")
        (:then
          (CallFunction|ExpandUIWidget _returnvalue)
          (if (not (Variables|Default|GetMusicPlaying))
            (Audio|PlaySound2D (.InstrumentMusic (Utilities|Struct|BreakInstrument_DataStructure _returnvalue)) 1.0 1.0 0.0 0 0)
            (Variables|Default|SetMusicPlaying true)))))
    (:UIActor_BP2
      (bind _returnvalue_2 (Utilities|GetDataTableRow "/Game/Instrument_dataTable.Instrument_dataTable" "Piano")
        (:then
          (CallFunction|ExpandUIWidget _returnvalue_2)
          (if (not (Variables|Default|GetMusicPlaying))
            (Audio|PlaySound2D (.InstrumentMusic (Utilities|Struct|BreakInstrument_DataStructure _returnvalue_2)) 1.0 1.0 0.0 0 0)
            (Variables|Default|SetMusicPlaying true)))))
    (:UIActor_BP3
      (bind _returnvalue_3 (Utilities|GetDataTableRow "/Game/Instrument_dataTable.Instrument_dataTable" "Trumpet")
        (:then
          (CallFunction|ExpandUIWidget _returnvalue_3)
          (if (not (Variables|Default|GetMusicPlaying))
            (Audio|PlaySound2D (.InstrumentMusic (Utilities|Struct|BreakInstrument_DataStructure _returnvalue_3)) 1.0 1.0 0.0 0 0)
            (Variables|Default|SetMusicPlaying true)))))))

(event Collision|EventActorEndOverlap
  (params (OtherActor :type Actor%20Object%20Reference))
  (Variables|Default|SetMusicPlaying false))

(event EventTick
  (params (DeltaSeconds :type Float%20%28single-precision%29)))

(event Collision|EventActorBeginOverlap
  (params (OtherActor :type Actor%20Object%20Reference)))

(event EventBeginPlay)

(fn ConstructionScript)

(fn ExpandUIWidget
  (params (Instrument_DataStructure :type Instrument%20Data%20Structure%20Structure%20%28by%20ref%29)))